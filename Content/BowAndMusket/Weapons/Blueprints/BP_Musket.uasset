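; Matchlock musket actor whose firing depends on an attached match rope and priming powder.
; Firing, unless reloading, animates the serpentine and after a short delay consumes the rope, then any powder, which triggers emitter, recoil and powder respawn calls.
; Separate events spawn and attach replacement rope and powder, and toggle the pan cover with a FlipFlop.
; Trigger and cover motion are driven by setting variables on the cached Animation Blueprint.
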(event `self.ReceiveBeginPlay`
  ;[1 1 1] Get Animation Blueprint Ref
  (bind _asmusket_anim_bp (cast `/Game/BowAndMusket/Weapons/Blueprints/Musket_AnimBP` (`SkeletalMeshComponent.GetAnimInstance` (`self.Frame`))))
  (set `self.Musket Anim BP` _asmusket_anim_bp))

(event `/Game/BowAndMusket/Interfaces/BPI_WeaponLogic.WeaponFire`
  (bind _musket_anim_bp (`self.Musket Anim BP`))
  (bind _attachedrope (`self.AttachedRope`))
  (bind _attachedpowder (`self.AttachedPowder`))
  ;[1 1 1] 머스킷 격발 준비과정
  (if (not (`self.IsReloading`))
    ;;[1 1 1] 격발시 용두가 내려가는 애니메이션 재생
    (set `/Game/BowAndMusket/Weapons/Blueprints/Musket_AnimBP.PlayFireAnimation` true _musket_anim_bp)
    (set `/Game/BowAndMusket/Weapons/Blueprints/Musket_AnimBP.TriggerRotationValue` (struct :`Roll` 40.0) _musket_anim_bp)
    (`KismetSystemLibrary.Delay` 0.2) ; 애니메이션 재생 시간
    (`/Engine/EditorBlueprintResources/StandardMacros.IsValid` _attachedrope ; 로프가 존재할경우
      (:`Is Valid`
        ;;[1 1 1] 로프 존재
        (`self.K2_DestroyActor` _attachedrope)
        (set `self.FiredRopeAttachable` true)
        (`/Engine/EditorBlueprintResources/StandardMacros.IsValid` _attachedpowder ; 화약접시의 화약 존재
          (:`Is Valid`
            (`self.K2_DestroyActor` _attachedpowder) ; 총에 부착된 화약 없애기
            (`self.SpawnEmitterandRecoil`)
            (`self.Respawn Powder`)))))))

(event `/Game/BowAndMusket/Interfaces/BPI_WeaponLogic.WeaponTriggerRelease`
  ;[1 1 1] 트리거에서 손을 땔시
  (set `/Game/BowAndMusket/Weapons/Blueprints/Musket_AnimBP.PlayFireAnimation` false (`self.Musket Anim BP`))
  (set `/Game/BowAndMusket/Weapons/Blueprints/Musket_AnimBP.TriggerRotationValue` (struct) (`self.Musket Anim BP`)))

(event `self.GetFiredRope`
  ;[1 1 1] 화승을 어태치한다
  (if (`self.FiredRopeAttachable`)
    (bind _returnvalue (`|SpawnActorFromClass` "/Game/BowAndMusket/Weapons/Blueprints/NotGuns/BP_Rope.BP_Rope_C" (`SceneComponent.GetSocketTransform` (`self.Frame`) "RopePosition" "RTS_World") "Undefined" "OverrideRootScale" null null))
    (bind _output_get (set `self.AttachedRope` _returnvalue))
    (`self.K2_AttachToComponent` _output_get (`self.Frame`) "RopePosition" "SnapToTarget" "SnapToTarget" "SnapToTarget" true)
    (set `self.FiredRopeAttachable` false)))

(event `self.RotatePowderCap`
  ;[1 1 1] 화약접시의 회전을 구현
  (`/Engine/EditorBlueprintResources/StandardMacros.FlipFlop`
    (:`A`
      (set `/Game/BowAndMusket/Weapons/Blueprints/Musket_AnimBP. FirecapRotationValue` (struct :`Yaw` -90.0) (`self.Musket Anim BP`))
      (set `self.PowderCapOpen` true))
    (:`B`
      (set `/Game/BowAndMusket/Weapons/Blueprints/Musket_AnimBP. FirecapRotationValue` (struct) (`self.Musket Anim BP`))
      (set `self.PowderCapOpen` false))))

(event `self.GetPowder`
  (bind _powderspawnloc (`self.PowderSpawnLoc`))
  (bind (_returnvalue_location _returnvalue_rotation) (`KismetMathLibrary.BreakTransform` (`SceneComponent.K2_GetComponentToWorld` _powderspawnloc)))
  ;[1 1 1] 화약접시에 화약을 스폰하는 로직
  (bind _returnvalue (`|SpawnActorFromClass` "/Game/BowAndMusket/Weapons/Blueprints/NotGuns/BP_GunPowder.BP_GunPowder_C" (`KismetMathLibrary.MakeTransform` _returnvalue_location _returnvalue_rotation) "Undefined" "OverrideRootScale" null null))
  (bind _output_get (set `self.AttachedPowder` _returnvalue))
  (`self.K2_AttachToComponent` _output_get _powderspawnloc "None" "SnapToTarget" "SnapToTarget" "SnapToTarget" true))

(fn `UserConstructionScript`
  (`SceneComponent.K2_AttachToComponent` (`self.PowderSpawnLoc`) (`self.TriggerBoxParent`) "None" "KeepRelative" "KeepRelative" "KeepRelative" true))