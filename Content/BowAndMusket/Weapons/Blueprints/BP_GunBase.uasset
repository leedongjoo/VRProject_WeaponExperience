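; Base Blueprint for musket-style guns, with trigger boxes for charging, grips, fire rope and powder.
; The construction script runs attachment on the trigger-box hierarchy, then destroys the second-grip, fire and powder triggers when their Allows flags are off.
; Events toggle fired-rope usability and ask the level's PowderReSpawnRocation actor to respawn powder.
; Powder cap, powder pickup and emitter/recoil events are empty stubs.
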(event `self.ReceiveBeginPlay`
  ;[1 1 1] BeginPlay
)

(event `/Game/BowAndMusket/Interfaces/BPI_WeaponLogic.WeaponFire`
  (set `self.IsFiredRopeUsable` false))

(event `RotatePowderCap`
  ;[1 1 1] Musket 사용 이벤트
)

(event `GetFiredRope`
  (set `self.IsFiredRopeUsable` true))

(event `GetPowder`)

(event `SpawnEmitterandRecoil`)

(event `Respawn Powder`
  ;[1 1 1] 총 다 쏘고 나서 화약을 리스폰한다
  (bind _returnvalue (`GameplayStatics.GetActorOfClass` "/Game/BowAndMusket/Blueprints/PowderReSpawnRocation.PowderReSpawnRocation_C"))
  (`/Engine/EditorBlueprintResources/StandardMacros.IsValid` _returnvalue
    (:`Is Valid`
      (`/Game/BowAndMusket/Blueprints/PowderReSpawnRocation.RespawnPowder` _returnvalue))
    (:`Is Not Valid`
      (`KismetSystemLibrary.PrintString` "밷"))))

(fn `NewFunction_0`)

(fn `UserConstructionScript`
  (`|ExecutionSequence`
    (:`then_0`
      (for _ (`|MakeArray` (`self.ChargingTrigger`) (`self.2ndGrab`) (`self.1ndGrab`) (`self.FireTrigger`) (`self.PowderTrigger`))
        (`SceneComponent.K2_AttachToComponent` (`self.TriggerBoxParent`) null "None" "KeepRelative" "KeepRelative" "KeepRelative" true)))
    (:`then_1`
      ;[1 1 1] 2Handed 그립 트리거 필요없으면 삭제
      (if (not (`self.Allows2HandedGrip`))
        (`ActorComponent.K2_DestroyComponent` (`self.2ndGrab`))))
    (:`then_2`
      ;[1 1 1] 화승 트리거 총기에 따라 필요없으면 삭제
      (if (not (`self.AllowsFireTrigger`))
        (`ActorComponent.K2_DestroyComponent` (`self.FireTrigger`))))
    (:`then_3`
      ;[1 1 1] 화약접시 트리거 총기에 따라 필요없으면 삭제
      (if (not (`self.AllowsPowderTrigger`))
        (`ActorComponent.K2_DestroyComponent` (`self.PowderTrigger`))))))