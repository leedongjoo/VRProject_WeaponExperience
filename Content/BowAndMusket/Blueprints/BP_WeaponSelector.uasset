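; BP_WeaponSelector is a weapon display actor that shows one selected weapon with title and information widgets and a spoken description.
; On BeginPlay it applies initial widget visibility, sets mesh and sound from the selected weapon's info struct, and passes itself to both widgets.
; Events toggle the info widget and narration, stopping other selectors' audio so only one plays.
; A timeline for moving the mesh exists but is never triggered.
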(event `/Game/BowAndMusket/Interfaces/BPI_WeaponSelector.WeaponInfoOn/Off`
  (params (`TurnWeaponInfo on/off` :type Boolean))
  ;[1 1 1] Weapon Info 창 켜고 끄기
  (`SceneComponent.SetVisibility` (`self.WeaponInfoWidget`) `TurnWeaponInfo on/off` false))

(event `/Game/BowAndMusket/Interfaces/BPI_WeaponSelector.WeaponPTSoundOn/Off`
  (params (PlaySound :type Boolean))
  ;[1 1 1] 무기 설명 사운드 토글
  (bind _outactors (`GameplayStatics.GetAllActorsOfClass` "BP_WeaponSelector_C"))
  (for _array_element _outactors
    (if (== _array_element self)
      (if PlaySound
        (bind _audio (`/Game/BowAndMusket/Blueprints/BP_WeaponSelector.Audio` _array_element))
        (`AudioComponent.Play` _audio 0.0)
        (else
          (`AudioComponent.Stop` _audio)))
      (else
        (bind _audio_2 (`/Game/BowAndMusket/Blueprints/BP_WeaponSelector.Audio` _array_element))
        (if (`AudioComponent.IsPlaying` _audio_2)
          (`AudioComponent.Stop` _audio_2))))))

(event `self.ReceiveBeginPlay`
  (`|ExecutionSequence`
    (:`then_0`
      ;[1 1 1] 위젯 비지빌리티 설정
      (`SceneComponent.SetVisibility` (`self.WeaponInfoWidget`) (`self.bWeaponInfoWidgetVisible`) false)
      (`SceneComponent.SetVisibility` (`self.WeaponTitleWidget`) (`self.bWeaponTitleWidgetVisible`) false))
    (:`then_1`
      (`self.Set Weapon Mesh`) ; 무기 메시 설정
      (`self.Set Weapon PTSound`) ; 무기 음성 설정
    )
    (:`then_2`
      ;[1 1 1] 셀렉터 레퍼런스를 위젯에 전달
      (bind _aswb_weapon_information (cast `/Game/BowAndMusket/UMG/WB_WeaponInformation` (`WidgetComponent.GetUserWidgetObject` (`self.WeaponInfoWidget`))))
      (set `/Game/BowAndMusket/UMG/WB_WeaponInformation.WeaponSelectorActor` self _aswb_weapon_information)
      (bind _aswb_weapon_title (cast `/Game/BowAndMusket/UMG/WB_WeaponTitle` (`WidgetComponent.GetUserWidgetObject` (`self.WeaponTitleWidget`))))
      (set `/Game/BowAndMusket/UMG/WB_WeaponTitle.WeaponSelectorActor` self _aswb_weapon_title))))

(fn `Set Weapon Mesh`
  (bind _returnvalue (select `/Game/BowAndMusket/Enums/E_Weapons` (`self.SelectedWeapon`) :`NewEnumerator0` (`.WeaponMesh_22_920A3BF54FDD0723E1184988ED7AA89D` (break `/Game/BowAndMusket/Structs/S_WeaponInformation` (`self.SeungJarGunInfo`))) :`NewEnumerator1` (`.WeaponMesh_22_920A3BF54FDD0723E1184988ED7AA89D` (break `/Game/BowAndMusket/Structs/S_WeaponInformation` (`self.BowInfo`))) :`NewEnumerator2` (`.WeaponMesh_22_920A3BF54FDD0723E1184988ED7AA89D` (break `/Game/BowAndMusket/Structs/S_WeaponInformation` (`self.MusketInfo`))) :`NewEnumerator3` (`.WeaponMesh_22_920A3BF54FDD0723E1184988ED7AA89D` (break `/Game/BowAndMusket/Structs/S_WeaponInformation` (`self.CannonBallInfo`)))))
  (`/Engine/EditorBlueprintResources/StandardMacros.IsValid` _returnvalue
    (:`Is Valid`
      (`StaticMeshComponent.SetStaticMesh` (`self.Weapon_Mesh`) _returnvalue))))

(fn `Set Weapon PTSound`
  (bind _returnvalue (select `/Game/BowAndMusket/Enums/E_Weapons` (`self.SelectedWeapon`) :`NewEnumerator0` (`.TtsSound_29_E713EC4344E7508F5740AE852303090D` (break `/Game/BowAndMusket/Structs/S_WeaponInformation` (`self.SeungJarGunInfo`))) :`NewEnumerator1` (`.TtsSound_29_E713EC4344E7508F5740AE852303090D` (break `/Game/BowAndMusket/Structs/S_WeaponInformation` (`self.BowInfo`))) :`NewEnumerator2` (`.TtsSound_29_E713EC4344E7508F5740AE852303090D` (break `/Game/BowAndMusket/Structs/S_WeaponInformation` (`self.MusketInfo`))) :`NewEnumerator3` (`.TtsSound_29_E713EC4344E7508F5740AE852303090D` (break `/Game/BowAndMusket/Structs/S_WeaponInformation` (`self.CannonBallInfo`)))))
  (`/Engine/EditorBlueprintResources/StandardMacros.IsValid` _returnvalue
    (:`Is Valid`
      (`AudioComponent.SetSound` (`self.Audio`) _returnvalue))))

(fn `UserConstructionScript`)